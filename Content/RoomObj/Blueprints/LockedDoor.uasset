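; A lockable room door that the player swings open or closed with the Interact input while inside its trigger box.
; Overlap enables input and shows a prompt widget, reading "The door is locked" when locked; otherwise it opens a gate that lets Interact through.
; Separate timelines lerp the door's yaw for opening and closing.
; Locked, closed and near-door flags serialize to a digit string, which SetProperties parses back.
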(event `InputAction|Interact` :consume false
  (params (Key :type "Key Structure"))
  (:`Pressed`
    (if (not (`self.IsDoorLocked`))
      (`/Engine/EditorBlueprintResources/StandardMacros.Gate` true :!label _label
        (:`Exit`
          (if (`self.IsDoorClosed`)
            (bind (_direction _open_close) (`Timeline|Door Open` :!via `PlayFromStart`)
              (:`Update`
                (`SceneComponent.K2_SetRelativeRotation` (`self.Door`) (`KismetMathLibrary.MakeRotator` 0.0 0.0 (`KismetMathLibrary.Lerp` (`self.Close Angle`) (`self.Open Angle`) _open_close)) false false))
              (:`Finished`
                (set `self.IsDoorClosed` false)))
            (else
              (bind (_direction_2 _open_close_2) (`Timeline|Timeline_0` :!via `ReverseFromEnd`)
                (:`Update`
                  (`SceneComponent.K2_SetRelativeRotation` (`self.Door`) (`KismetMathLibrary.MakeRotator` 0.0 0.0 (`KismetMathLibrary.Lerp` (`self.Close Angle`) (`self.Open Angle`) _open_close_2)) false false))
                (:`Finished`
                  (set `self.IsDoorClosed` true))))))))))

(event `self.Box.OnComponentBeginOverlap`
  (params (OverlappedComponent :type "PrimitiveComponent Object Reference") (OtherActor :type "Actor Object Reference") (OtherComp :type "PrimitiveComponent Object Reference") (OtherBodyIndex :type Integer) (bFromSweep :type Boolean) (SweepResult :type "HitResult Structure (by ref)"))
  ;[1 1 1] Proximity Verification
  (set `self.IsNearDoor` true)
  (`self.EnableInput` (`GameplayStatics.GetPlayerController` 0))
  (if (`self.IsDoorLocked`)
    (cast `/Game/TP_Character` OtherActor)
    (bind _returnvalue (`|CreateWidget` "/Game/Widgets/InteractPromptWidget.InteractPromptWidget_C"))
    (`EditableTextBox.SetText` (`/Game/Widgets/InteractPromptWidget.EditableTextBox_271` _returnvalue) "The door is locked")
    (`UserWidget.AddToViewport` _returnvalue 0)
    (else
      (cast `/Game/TP_Character` OtherActor)
      (bind _returnvalue_2 (`|CreateWidget` "/Game/Widgets/InteractPromptWidget.InteractPromptWidget_C"))
      (`UserWidget.AddToViewport` _returnvalue_2 0)
      (goto _label :!via `Open`))))

(event `self.Box.OnComponentEndOverlap`
  (params (OverlappedComponent :type "PrimitiveComponent Object Reference") (OtherActor :type "Actor Object Reference") (OtherComp :type "PrimitiveComponent Object Reference") (OtherBodyIndex :type Integer))
  ;[1 1 1] Proximity Verification
  (set `self.IsNearDoor` false)
  (`self.DisableInput` (`GameplayStatics.GetPlayerController` 0))
  (if (`self.IsDoorLocked`)
    (cast `/Game/TP_Character` OtherActor)
    (`Widget.RemoveFromParent` (stale `self.Box.OnComponentBeginOverlap` _returnvalue))
    (else
      (cast `/Game/TP_Character` OtherActor)
      (`Widget.RemoveFromParent` (stale `self.Box.OnComponentBeginOverlap` _returnvalue_2))
      (goto _label :!via `Close`))))

(event `/Game/InteractableInterface.SetProperties`
  (params (Properties :type String))
  (set `self.IsDoorLocked` (`KismetMathLibrary.Conv_IntToBool` (- (`KismetStringLibrary.GetCharacterAsNumber` Properties) 48)))
  (set `self.IsDoorClosed` (`KismetMathLibrary.Conv_IntToBool` (- (`KismetStringLibrary.GetCharacterAsNumber` Properties 1) 48)))
  (set `self.IsNearDoor` (`KismetMathLibrary.Conv_IntToBool` (- (`KismetStringLibrary.GetCharacterAsNumber` Properties 2) 48))))

(fn `CloseDoor`
  (set `self.IsDoorClosed` true)
  (`SceneComponent.K2_SetRelativeRotation` (`self.Door`) (`KismetMathLibrary.MakeRotator` 0.0 0.0 (`self.Close Angle`)) false false))

(fn `GetObjectProprieties`
  (returns (Proprieties :type String))
  (return (`KismetStringLibrary.Concat_StrStr` (`KismetStringLibrary.Conv_IntToString` (`KismetMathLibrary.Conv_BoolToInt` (`self.IsDoorLocked`))) (`KismetStringLibrary.Conv_IntToString` (`KismetMathLibrary.Conv_BoolToInt` (`self.IsDoorClosed`))) (`KismetStringLibrary.Conv_IntToString` (`KismetMathLibrary.Conv_BoolToInt` (`self.IsNearDoor`))))))

(fn `Open Door`
  (set `self.IsDoorClosed` false)
  (`SceneComponent.K2_SetRelativeRotation` (`self.Door`) (`KismetMathLibrary.MakeRotator` 0.0 0.0 (`self.Open Angle`)) false false))

(fn `UserConstructionScript`)