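; Interactable tree actor that toggles between normal and altered size, with a matching color change, when the player presses Interact nearby.
; A box trigger enables input and opens a gate on overlap, showing a prompt widget for TP_Character, and undoes this on exit.
; Separate timelines scale the actor up or back down, while a third plays or reverses to fade a dynamic material's Color parameter.
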(event `self.ReceiveBeginPlay`
  ;[1 1 1] Scale and Color Modification
  (bind _returnvalue (`PrimitiveComponent.CreateDynamicMaterialInstance` (`self.StaticMesh`) 0 null "None")))

(event `InputAction|Interact`
  (params (Key :type "Key Structure"))
  (:`Pressed`
    (`/Engine/EditorBlueprintResources/StandardMacros.Gate` true :!label _label
      (:`Exit`
        ;[1 1 1] Scale and Color Modification
        (if (and (`self.IsNearBush`) (`self.IsNormalSize`))
          (bind (_direction _scale_increase) (`Timeline|Timeline_1` :!via `PlayFromStart`)
            (:`Update`
              (`self.SetActorScale3D` _scale_increase)
              (set `self.IsNormalSize` false)
              (bind (_direction_2 _color_fade) (`Timeline|Timeline_0` :!label _label_2)
                (:`Update`
                  (`MaterialInstanceDynamic.SetVectorParameterValue` (stale `self.ReceiveBeginPlay` _returnvalue) "Color" _color_fade)))))
          (elif (not (`self.IsNormalSize`))
            (bind (_direction_3 _scale_decrease) (`Timeline|Timeline_2` :!via `PlayFromStart`)
              (:`Update`
                (`self.SetActorScale3D` _scale_decrease)
                (set `self.IsNormalSize` true)
                (goto _label_2 :!via `Reverse`)))))))))

(event `self.Box.OnComponentBeginOverlap`
  (params (OverlappedComponent :type "PrimitiveComponent Object Reference") (OtherActor :type "Actor Object Reference") (OtherComp :type "PrimitiveComponent Object Reference") (OtherBodyIndex :type Integer) (bFromSweep :type Boolean) (SweepResult :type "HitResult Structure (by ref)"))
  ;[1 1 1] Proximity Verification
  (set `self.IsNearBush` true)
  (`self.EnableInput` (`GameplayStatics.GetPlayerController` 0))
  (cast `/Game/TP_Character` OtherActor)
  (bind _returnvalue (`|CreateWidget` "/Game/Widgets/InteractPromptWidget.InteractPromptWidget_C"))
  (`UserWidget.AddToViewport` _returnvalue 0)
  (goto _label :!via `Open`))

(event `self.Box.OnComponentEndOverlap`
  (params (OverlappedComponent :type "PrimitiveComponent Object Reference") (OtherActor :type "Actor Object Reference") (OtherComp :type "PrimitiveComponent Object Reference") (OtherBodyIndex :type Integer))
  ;[1 1 1] Proximity Verification
  (set `self.IsNearBush` false)
  (`self.DisableInput` (`GameplayStatics.GetPlayerController` 0))
  (cast `/Game/TP_Character` OtherActor)
  (`Widget.RemoveFromParent` (stale `self.Box.OnComponentBeginOverlap` _returnvalue))
  (goto _label :!via `Close`))

(fn `UserConstructionScript`)