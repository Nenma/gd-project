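; LevelManager is an overlap-triggered actor that advances the game to the next level in its Levels list.
; On any actor overlap, it looks up the current level name in the list and opens the following entry, doing nothing at the last one.
; An unlisted current level resolves to the first entry.
; The transition requires the game instance to be a TP_GameInstance, though nothing is read from it.
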(event `self.ReceiveActorBeginOverlap`
  (params (OtherActor :type "Actor Object Reference"))
  (bind _levels (`self.Levels`))
  (bind _returnvalue (`GameplayStatics.GetCurrentLevelName` true))
  (bind _returnvalue_2 (+ (`KismetArrayLibrary.Array_Find` _levels (`KismetStringLibrary.Conv_StringToName` _returnvalue)) 1))
  (if (< _returnvalue_2 (`KismetArrayLibrary.Array_Length` _levels))
    (cast `/Game/TP_GameInstance` (`GameplayStatics.GetGameInstance`))
    (`GameplayStatics.OpenLevel` (`|GetArrayItem` _levels _returnvalue_2))))

(fn `UserConstructionScript`)