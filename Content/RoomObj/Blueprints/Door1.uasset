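; Door1 is an interactable swinging door that the player opens and closes with the Interact input when nearby.
; A Box overlap toggles player input, while a successful cast of the overlapping actor also shows or removes a prompt widget and opens or closes a Gate.
; Interact passes through that Gate and branches on IsDoorClosed, playing one timeline forward or another in reverse to lerp Door yaw between CloseAngle and OpenAngle.
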(event `InputAction|Interact` :consume false
  (params (Key :type "Key Structure"))
  (:`Pressed`
    (`/Engine/EditorBlueprintResources/StandardMacros.Gate` true :!label _label
      (:`Exit`
        (if (`self.IsDoorClosed`)
          (bind (_direction _open_close) (`Timeline|Door Open` :!via `PlayFromStart`)
            (:`Update`
              (`SceneComponent.K2_SetRelativeRotation` (`self.Door`) (`KismetMathLibrary.MakeRotator` 0.0 0.0 (`KismetMathLibrary.Lerp` (`self.Close Angle`) (`self.Open Angle`) _open_close)) false false))
            (:`Finished`
              (set `self.IsDoorClosed` false)))
          (else
            (bind (_direction_2 _open_close_2) (`Timeline|Timeline_0` :!via `ReverseFromEnd`)
              (:`Update`
                (`SceneComponent.K2_SetRelativeRotation` (`self.Door`) (`KismetMathLibrary.MakeRotator` 0.0 0.0 (`KismetMathLibrary.Lerp` (`self.Close Angle`) (`self.Open Angle`) _open_close_2)) false false))
              (:`Finished`
                (set `self.IsDoorClosed` true)))))))))

(event `self.Box.OnComponentBeginOverlap`
  (params (OverlappedComponent :type "PrimitiveComponent Object Reference") (OtherActor :type "Actor Object Reference") (OtherComp :type "PrimitiveComponent Object Reference") (OtherBodyIndex :type Integer) (bFromSweep :type Boolean) (SweepResult :type "HitResult Structure (by ref)"))
  ;[1 1 1] Proximity Verification
  (set `self.IsNearDoor` true)
  (`self.EnableInput` (`GameplayStatics.GetPlayerController` 0))
  (cast `` OtherActor)
  (bind _returnvalue (`|CreateWidget` "/Game/Widgets/InteractPromptWidget.InteractPromptWidget_C"))
  (`UserWidget.AddToViewport` _returnvalue 0)
  (goto _label :!via `Open`))

(event `self.Box.OnComponentEndOverlap`
  (params (OverlappedComponent :type "PrimitiveComponent Object Reference") (OtherActor :type "Actor Object Reference") (OtherComp :type "PrimitiveComponent Object Reference") (OtherBodyIndex :type Integer))
  ;[1 1 1] Proximity Verification
  (set `self.IsNearDoor` false)
  (`self.DisableInput` (`GameplayStatics.GetPlayerController` 0))
  (cast `` OtherActor)
  (`Widget.RemoveFromParent` (stale `self.Box.OnComponentBeginOverlap` _returnvalue))
  (goto _label :!via `Close`))

(fn `UserConstructionScript`)