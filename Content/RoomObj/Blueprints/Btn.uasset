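; Interactable button actor that unlocks a LockedDoor sharing the button's first actor tag.
; Box overlap enables player input, finds the first matching door and, if it is locked and a TP_Character entered, shows an interact prompt and opens a Gate.
; Pressing Interact through the Gate unlocks the door, removes the prompt and closes the Gate.
; Leaving the box disables input and, for a TP_Character, clears the prompt and Gate.
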(event `InputAction|Interact`
  (params (Key :type "Key Structure"))
  (:`Pressed`
    (`/Engine/EditorBlueprintResources/StandardMacros.Gate` true :!label _label
      (:`Exit`
        (set `/Game/RoomObj/Blueprints/LockedDoor.IsDoorLocked` false (`|GetArrayItem` (stale `self.Box.OnComponentBeginOverlap` _outactors)))
        (`Widget.RemoveFromParent` (stale `self.Box.OnComponentBeginOverlap` _returnvalue) :!label _label_2)
        (goto _label :!via `Close`)))))

(event `self.Box.OnComponentBeginOverlap`
  (params (OverlappedComponent :type "PrimitiveComponent Object Reference") (OtherActor :type "Actor Object Reference") (OtherComp :type "PrimitiveComponent Object Reference") (OtherBodyIndex :type Integer) (bFromSweep :type Boolean) (SweepResult :type "HitResult Structure (by ref)"))
  ;[1 1 1] Proximity Verification
  (set `self.IsNearBtn` true)
  (`self.EnableInput` (`GameplayStatics.GetPlayerController` 0))
  (bind _outactors (`GameplayStatics.GetAllActorsOfClassWithTag` "/Game/RoomObj/Blueprints/LockedDoor.LockedDoor_C" (`|GetArrayItem` (`self.Tags`))))
  (if (`/Game/RoomObj/Blueprints/LockedDoor.IsDoorLocked` (`|GetArrayItem` _outactors))
    (cast `/Game/TP_Character` OtherActor)
    (bind _returnvalue (`|CreateWidget` "/Game/Widgets/InteractPromptWidget.InteractPromptWidget_C"))
    (`UserWidget.AddToViewport` _returnvalue 0)
    (goto _label :!via `Open`)))

(event `self.Box.OnComponentEndOverlap`
  (params (OverlappedComponent :type "PrimitiveComponent Object Reference") (OtherActor :type "Actor Object Reference") (OtherComp :type "PrimitiveComponent Object Reference") (OtherBodyIndex :type Integer))
  ;[1 1 1] Proximity Verification
  (set `self.IsNearBtn` false)
  (`self.DisableInput` (`GameplayStatics.GetPlayerController` 0))
  (cast `/Game/TP_Character` OtherActor)
  (goto _label_2))

(fn `UserConstructionScript`)