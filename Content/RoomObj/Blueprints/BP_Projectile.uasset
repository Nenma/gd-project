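; Projectile actor that bounces off Mirror actors or rotates them, and is destroyed on hitting a CollisionBox.
; On overlap, a dot product against the mirror's facing picks the outcome: one side turns the mirror 45 degrees, updates its reflection directions and destroys the projectile.
; The other decrements MirrorsToHit, snaps the projectile to the mirror's box and re-orients it with a reflection vector.
; Angle checks only print debug text; velocity redirects are disconnected.
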(event `self.ReceiveActorBeginOverlap`
  (params (OtherActor :type "Actor Object Reference"))
  (bind _asmirror (cast `/Game/ThirdPersonBP/Blueprints/Mirror` OtherActor)
    (:`then`
      (bind _returnvalue (`self.K2_GetActorRotation` _asmirror))
      ;[1 1 1] Check if in front or behind mirror
      (if (< (`KismetMathLibrary.Dot_VectorVector` (`self.GetActorForwardVector`) (`KismetMathLibrary.GreaterGreater_VectorRotator` (0.0 -1.0 0.0) _returnvalue)) 0.0)
        (bind (_returnvalue_roll _returnvalue_pitch _returnvalue_yaw) (`KismetMathLibrary.BreakRotator` (`self.K2_GetActorRotation` _asmirror)))
        (bind _returnvalue_2 (+ _returnvalue_yaw 45.0))
        ;[1 1 1] Rotate Mirror
        (`self.K2_SetActorRotation` _asmirror (`KismetMathLibrary.MakeRotator` _returnvalue_roll _returnvalue_pitch _returnvalue_2) false)
        (`self.K2_DestroyActor`)
        (set `/Game/ThirdPersonBP/Blueprints/Mirror.reflectionDirection` (`KismetMathLibrary.GreaterGreater_VectorRotator` (`/Game/ThirdPersonBP/Blueprints/Mirror.reflectionDirection` _asmirror) (`KismetMathLibrary.MakeRotator` _returnvalue_roll 0.0 _returnvalue_2)) _asmirror)
        (set `/Game/ThirdPersonBP/Blueprints/Mirror.reflectionDirection2` (`KismetMathLibrary.GreaterGreater_VectorRotator` (`/Game/ThirdPersonBP/Blueprints/Mirror.reflectionDirection2` _asmirror) (`KismetMathLibrary.MakeRotator` _returnvalue_roll 0.0 _returnvalue_2)) _asmirror)
        (else
          (`/Engine/EditorBlueprintResources/StandardMacros.DecrementInt` (`self.MirrorsToHit`)
            (:`  `
              ;[1 1 1] Set new position & rotation of bullet
              (`self.K2_SetActorLocation` (`SceneComponent.K2_GetComponentLocation` (`/Game/ThirdPersonBP/Blueprints/Mirror.Box` _asmirror)))
              (`self.K2_SetActorRotation` (`KismetMathLibrary.MakeRotFromZ` (`KismetMathLibrary.GetReflectionVector` (`self.GetActorForwardVector`) (`KismetMathLibrary.GreaterGreater_VectorRotator` (0.0 1.0 0.0) _returnvalue))) true)
              (bind _returnvalue_3 (`KismetMathLibrary.DegAcos` (`KismetMathLibrary.Dot_VectorVector` (`self.GetActorForwardVector`) (`/Game/ThirdPersonBP/Blueprints/Mirror.reflectionDirection` _asmirror))))
              (`KismetSystemLibrary.PrintString` (`KismetStringLibrary.Conv_DoubleToString` _returnvalue_3))
              (if (> _returnvalue_3 45.0)
                (`KismetSystemLibrary.PrintString` "Approximate direct")
                (else
                  (`KismetSystemLibrary.PrintString` "Aproximate inverse"))))))))
    (:`CastFailed`
      (cast `/Game/ThirdPersonBP/Blueprints/CollisionBox` OtherActor)
      (`self.K2_DestroyActor`))))

(fn `UserConstructionScript`)